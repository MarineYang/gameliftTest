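; Player controller that handles player session acceptance and logout, apparently for a dedicated server test.
; PlayerAccept reads the session ID from BP_GameInstance and passes it to AcceptPlayerSessionId, which stores it and calls AcceptGameSession on DediTestGameMode.
; LogoutPlayer hands the stored ID to the game instance's LogoutProcess.
; Failed casts in the accept flow only print debug messages.
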(event Custom|PlayerAccept
  (bind _asbp_game_instance (Utilities|Casting|CastToBP_GameInstance (Game|GetGameInstance))
    (:then
      (bind _output_get (Variables|Default|SetPlayerSessionId (Variables|/Game/Blueprints/BP_GameInstance.BP_GameInstance_C|GetPlayerSessionID _asbp_game_instance)))
      (CallFunction|AcceptPlayerSessionId _output_get))
    (:CastFailed
      (Development|PrintString "Fail to BP_DediTestGameInstance Casting in BP_PlayerController"))))

(event Custom|AcceptPlayerSessionId
  (params (PlayerSessionId :type String))
  (bind _asdedi_test_game_mode (Utilities|Casting|CastToDediTestGameMode (Game|GetGameMode))
    (:then
      (Variables|Default|SetPlayerSessionId PlayerSessionId)
      (Class|DediTestGameMode|AcceptGameSession _asdedi_test_game_mode PlayerSessionId)
      (Development|PrintString "Accept Player ! "))
    (:CastFailed
      (Development|PrintString "DediTestGameMode Cast Faild in BP_PlayerController"))))

(event Custom|LogoutPlayer
  (bind _asbp_game_instance (Utilities|Casting|CastToBP_GameInstance (Game|GetGameInstance)))
  (Class|DediGameInstance|LogoutProcess _asbp_game_instance (Variables|Default|GetPlayerSessionId)))

(fn ConstructionScript)